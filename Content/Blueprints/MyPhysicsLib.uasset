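; Blueprint function library of visibility helpers for line-of-sight and on-screen checks.
; Line of sight requires a Camera-channel trace to the actor's location to hit that actor, with a variant between two actors that ignores the source.
; IsActorOnScreen approximates player 0's view frustum as an FOV cone, using a dot-product test on the actor's position only, and traces only when that passes.
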(fn `DoesLosBetweenActorsExist`
  (params (FromActor :type "Actor Object Reference") (ToActor :type "Actor Object Reference") (ActorsToIgnore :type "Array of Actor Object Reference"))
  (returns (LosExists :type Boolean))
  (`KismetArrayLibrary.Array_Add` (`local.ActorsToIgnore`) (`local.FromActor`))
  (return (`self.DoesLosToActorFromPosExist` (`Actor.K2_GetActorLocation` (`local.FromActor`)) (`local.ToActor`) (`local.ActorsToIgnore`) (`local.__WorldContext`))))

(fn `DoesLosToActorFromPosExist`
  (params (Pos :type "Vector Structure") (ToActor :type "Actor Object Reference") (ActorsToIgnore :type "Array of Actor Object Reference"))
  (returns (LosExists :type Boolean))
  (bind _outhit (`KismetSystemLibrary.LineTraceSingle` (`local.__WorldContext`) (`local.Pos`) (`Actor.K2_GetActorLocation` (`local.ToActor`)) "TraceTypeQuery2" false (`local.ActorsToIgnore`) "None" false))
  (bind (_bblockinghit _binitialoverlap _time _distance _location _impactpoint _normal _impactnormal _physmat _hitactor) (`GameplayStatics.BreakHitResult` _outhit))
  (return (and _bblockinghit (== (`local.ToActor`) _hitactor))))

(fn `IsActorOnScreen`
  (params (Actor :type "Actor Object Reference"))
  (returns (IsOnScreen :type Boolean))
  (bind _returnvalue (`GameplayStatics.GetPlayerCameraManager` (`local.__WorldContext`)))
  (if (`self.IsPositionInCone` (`Actor.K2_GetActorLocation` (`local.Actor`)) (`PlayerCameraManager.GetCameraLocation` _returnvalue) (`SceneComponent.GetForwardVector` (`PlayerCameraManager.TransformComponent` _returnvalue)) (`KismetMathLibrary.DegreesToRadians` (`PlayerCameraManager.GetFOVAngle` _returnvalue)) (`local.__WorldContext`))
    (return (`self.DoesLosToActorFromPosExist` (`PlayerCameraManager.GetCameraLocation` (`GameplayStatics.GetPlayerCameraManager` (`local.__WorldContext`))) (`local.Actor`) (`|MakeArray` null :!type "Actor Object Reference") (`local.__WorldContext`)))
    (else
      (return false) ; Don't bother raycasting if\nthe first condition isn't met\nanyways.
    )))

(fn `IsPositionInCone`
  (params (TargetPos :type "Vector Structure") (Peak :type "Vector Structure") (Dir :type "Vector Structure") (OpeningInRads :type "Float (double-precision)"))
  (returns (IsInCone :type Boolean))
  (return (>= (`KismetMathLibrary.Dot_VectorVector` (`KismetMathLibrary.Normal` (- (`local.TargetPos`) (`local.Peak`))) (`KismetMathLibrary.Normal` (`local.Dir`))) (`KismetMathLibrary.Cos` (* (`local.OpeningInRads`) 0.5)))))